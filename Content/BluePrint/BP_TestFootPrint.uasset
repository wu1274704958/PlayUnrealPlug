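; Test Blueprint that exercises footprint drawing through a FootPrintComponent.
; The construction script caches the first FootPrintComponent found on it, if any.
; Tick calls DrawFootPrint every frame, and pressing W triggers the same call after printing a debug string that mislabels the key as P.
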(event `self.ReceiveTick`
  (params (DeltaSeconds :type "Float (single-precision)"))
  (`FootPrintComponent.DrawFootPrint` (`self.FootPrintComponent`) :!label _label))

(event `Key|W`
  (params (Key :type "Key Structure"))
  (:`Pressed`
    (`KismetSystemLibrary.PrintString` "Key P pressed")
    (goto _label)))

(fn `UserConstructionScript`
  (bind _returnvalue (`self.K2_GetComponentsByClass` self "/Script/TestPlug.FootPrintComponent"))
  (if (>= (`KismetArrayLibrary.Array_Length` _returnvalue) 1)
    (set `self.FootPrintComponent` (`|GetArrayItem` _returnvalue))))
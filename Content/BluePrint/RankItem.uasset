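; RankItem is a 3D leaderboard entry actor showing a player's name, score, circular icon and crown.
; SetData fills the texts and downloads the icon from a path into a dynamic material's texture parameter.
; Tick spins the crown and sways the icon's yaw on an offset sine of elapsed time.
; The root starts lowered by AniDistance; a timeline drives its height for the start animation, which can be stopped.
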(event `PlayStartAnimation`
  (bind (_direction `_新建轨道_2`) (`Timeline|时间轴_0` :!via `PlayFromStart` :!label _label)
    (:`Update`
      (`SceneComponent.K2_SetRelativeLocationAndRotation` :`self` (`self.Root`) :`NewLocation` (`KismetMathLibrary.MakeVector` 0.0 0.0 (* (- `_新建轨道_2` 1.0) (`self.AniDistance`)))))))

(event `StopStartAnimation`
  (goto _label :!via `Stop`))

(event `DownloadIcon`
  (bind _texture (`AsyncTaskDownloadImage.DownloadImage` (`self.IconPath`))
    (:`OnSuccess`
      (`MaterialInstanceDynamic.SetTextureParameterValue` (`self.IconDynMaterial`) "Src" _texture))
    (:`OnFail`
      (`KismetSystemLibrary.PrintString` "下载失败"))))

(event `self.ReceiveBeginPlay`
  (bind _returnvalue (`PrimitiveComponent.CreateDynamicMaterialInstance` (`self.icon`) 0 "/Game/Materials/M_CircleIcon.M_CircleIcon" "None"))
  (set `self.IconDynMaterial` _returnvalue)
  (`self.RestRootPos`))

(event `self.ReceiveActorBeginOverlap`
  (params (OtherActor :type "Actor Object Reference")))

(event `self.ReceiveTick`
  (params (DeltaSeconds :type "Float (single-precision)"))
  (`self.RotateCrown` DeltaSeconds)
  (`self.RotateIcon` 0.0)
  (set `self.ElapsedTime` (+ (`self.ElapsedTime`) DeltaSeconds)))

(fn `PlayStartAni`
  (`self.PlayStartAnimation`))

(fn `RestRootPos`
  (`SceneComponent.K2_SetRelativeLocationAndRotation` :`self` (`self.Root`) :`NewLocation` (`KismetMathLibrary.MakeVector` 0.0 0.0 (* (`self.AniDistance`) -1.0))))

(fn `RotateCrown`
  (params (delta :type "Float (double-precision)"))
  (`SceneComponent.K2_AddLocalRotation` (`self.crown`) (`KismetMathLibrary.MakeRotator` 0.0 0.0 (* delta (`self.CrownRotateSpeed`))) false false))

(fn `RotateIcon`
  (params (delta :type "Float (double-precision)"))
  (bind _icon (`self.icon`))
  (bind _returnvalue_roll (`KismetMathLibrary.BreakRotator` (`SceneComponent.K2_GetComponentRotation` _icon)))
  (`SceneComponent.K2_SetWorldRotation` _icon (`KismetMathLibrary.MakeRotator` _returnvalue_roll 0.0 (+ (* (`KismetMathLibrary.Sin` (+ (`self.ElapsedTime`) (`self.IconZRoateAdd1`))) (`self.IconZRotateSpeed`)) (`self.IconZRoateAdd2`))) false false))

(fn `SetData`
  (params (name :type String) (score :type Integer) (iconPath :type String))
  (set `Text3DComponent.Text` (`KismetTextLibrary.Conv_StringToText` name) (`self.name`))
  (set `Text3DComponent.Text` (`KismetTextLibrary.Conv_StringToText` (`KismetStringLibrary.Conv_IntToString` score)) (`self.score`))
  (set `self.IconPath` iconPath)
  (`self.DownloadIcon`))

(fn `StopStartAni`
  (`self.StopStartAnimation`))

(fn `UserConstructionScript`)
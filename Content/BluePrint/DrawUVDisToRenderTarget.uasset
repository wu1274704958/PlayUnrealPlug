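; Actor Blueprint that draws a lens-distortion UV displacement map into a render target, with keyboard control over the distortion.
; Pressing W or S raises or lowers the K1 coefficient by a fixed increment, while K2 has no input binding.
; Every Tick clears the render target and redraws it from a camera model built with K1 and K2, so only the latest values appear.
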(event `Key|W`
  (params (Key :type "Key Structure"))
  ;[1 1 1] 增加（W）或降低（S）UV置换
  (:`Pressed`
    (set `self.K1` (+ (`self.K1`) (`self.inc`)))))

(event `Key|S`
  (params (Key :type "Key Structure"))
  ;[1 1 1] 增加（W）或降低（S）UV置换
  (:`Pressed`
    (set `self.K1` (+ (`self.K1`) (* (`self.inc`) -1.0)))))

(event `self.ReceiveTick`
  (params (DeltaSeconds :type "Float (single-precision)"))
  ;[1 1 1] 确保仅绘制最新K1和K2输入值
  (`KismetRenderingLibrary.ClearRenderTarget2D` "/Game/RT_00.RT_00")
  (`FooBlueprintLibrary.DrawUVDisplacementToRenderTarget` (make `FooCameraModel` (`self.K1`) (`self.K2`)) 1.0 1.0 1.0 "/Game/RT_00.RT_00"))

(fn `UserConstructionScript`)